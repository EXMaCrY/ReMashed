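; BP_LaserSightWeapon is a weapon item Blueprint that carries a laser sight and exposes the point it targets.
; GetLaserSightTarget casts the LaserSightActor child actor to BP_LaserSight and returns the result of its GetTargetPoint.
; The event graph holds only disabled stubs, and the construction script just calls the parent.
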(event EventBeginPlay
  (|CallParentFunction) ; This node is disabled and will not be called.\nDrag off pins to build functionality.
)

(event Collision|EventActorBeginOverlap
  (params (OtherActor :type Actor%20Object%20Reference))
  (|CallParentFunction OtherActor) ; This node is disabled and will not be called.\nDrag off pins to build functionality.
)

(event EventTick
  (params (DeltaSeconds :type Float%20%28single-precision%29))
  (|CallParentFunction DeltaSeconds) ; This node is disabled and will not be called.\nDrag off pins to build functionality.
)

(fn ConstructionScript
  (|CallParentFunction))

(fn GetLaserSightTarget
  (bind _asbp_laser_sight (Utilities|Casting|CastToBP_LaserSight (Variables|/Script/Engine.ChildActorComponent|GetChildActor (Variables|Default|GetLaserSightActor))))
  (bind _targetpoint (Default|GetTargetPoint _asbp_laser_sight))
  (return _targetpoint))