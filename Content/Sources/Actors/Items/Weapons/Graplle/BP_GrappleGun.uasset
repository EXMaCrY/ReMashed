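; Grapple gun weapon for wheeled vehicles that fires a hook on a cable and drags the shooter and the hit vehicle together.
; On use, it attaches the cable to the BP_Hook child actor's projectile mesh and launches it by physics impulse toward the laser-sight target.
; A vehicle hit starts a short looping timer applying opposite, distance-scaled forces to both vehicles, then the gun destroys itself.
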(event Custom|OnArrowBeginOverlap
  (params (OverlappedComponent :type Primitive%20Component%20Object%20Reference) (OtherActor :type Actor%20Object%20Reference) (OtherComp :type Primitive%20Component%20Object%20Reference) (OtherBodyIndex :type Integer) (bFromSweep :type Boolean) (SweepResult :type Hit%20Result%20Structure%20%28by%20ref%29))
  (bind _hook (Variables|Default|GetHook))
  (bind _target (Variables|/Game/Sources/Actors/Items/Projectiles/BP_Base_Projectile.BP_Base_Projectile_C|GetTarget _hook))
  (if (Utilities|IsValid _target)
    (bind _aswheeled_vehicle_pawn (Utilities|Casting|CastToWheeledVehiclePawn _target))
    (Variables|Default|SetTargetVehicle _aswheeled_vehicle_pawn)
    (bind _returnvalue (Utilities|Time|SetTimerbyEvent (delegate Custom|PullVehicles) 0.05 true))
    (Utilities|FlowControl|Delay 1.5)
    (Utilities|Time|ClearandInvalidateTimerbyHandle _returnvalue)
    (Actor|DestroyActor)
    (else
      (Utilities|FlowControl|Delay 1.0)
      (Actor|DestroyActor))))

(event Custom|PullVehicles
  (CallFunction|CalculateForceVector (Variables|Default|GetOwnerVehicle) (Variables|Default|GetTargetVehicle)))

(event EventBeginPlay
  (|CallParentFunction)
  (bind _asbp_hook (Utilities|Casting|CastToBP_Hook (Variables|/Script/Engine.ChildActorComponent|GetChildActor (Variables|Default|GetArrow))))
  (Variables|Default|SetHook _asbp_hook)
  (Collision|AssignOnComponentBeginOverlap (Variables|/Game/Sources/Actors/Items/Projectiles/BP_Base_Projectile.BP_Base_Projectile_C|GetCollision _asbp_hook) (delegate Custom|OnArrowBeginOverlap)))

(event Collision|EventActorBeginOverlap
  (params (OtherActor :type Actor%20Object%20Reference))
  (|CallParentFunction OtherActor) ; This node is disabled and will not be called.\nDrag off pins to build functionality.
)

(event EventTick
  (params (DeltaSeconds :type Float%20%28single-precision%29))
  (|CallParentFunction DeltaSeconds)
  (Variables|/Script/CableComponent.CableComponent|SetCableLength (Variables|Default|GetCable) (Math|Vector|Distance(Vector) (Transformation|GetWorldLocation (Variables|Default|GetCable)) (Transformation|GetWorldLocation (Variables|Default|GetArrow)))))

(event EventOnUse
  (|CallParentFunction)
  (bind _aswheeled_vehicle_pawn (Utilities|Casting|CastToWheeledVehiclePawn (Components|GetOwner)))
  (Variables|Default|SetOwnerVehicle _aswheeled_vehicle_pawn))

(fn ConstructionScript
  (|CallParentFunction))

(fn Use
  (|CallParentFunction)
  (CallFunction|InitComponents)
  (CallFunction|ShootArrow))

(fn InitComponents
  (bind _hook (Variables|Default|GetHook))
  (bind _projectilemesh (Variables|/Game/Sources/Actors/Items/Projectiles/BP_Base_Projectile.BP_Base_Projectile_C|GetProjectileMesh _hook))
  (Variables|/Script/Engine.PrimitiveComponent|SetbGenerateOverlapEvents (Variables|/Game/Sources/Actors/Items/Projectiles/BP_Base_Projectile.BP_Base_Projectile_C|GetCollision _hook) true)
  (Class|CableComponent|SetAttachEndtoComponent (Variables|Default|GetCable) _projectilemesh "Rope")
  (Physics|SetSimulatePhysics _projectilemesh true))

(fn ShootArrow
  (bind _targetpoint (CallFunction|GetLaserSightTarget))
  (Physics|AddImpulse (Variables|/Game/Sources/Actors/Items/Projectiles/BP_Base_Projectile.BP_Base_Projectile_C|GetProjectileMesh (Variables|Default|GetHook)) (* (Math|Vector|Normalize (- _targetpoint (Transformation|GetWorldLocation (Variables|Default|GetArrow)))) 1.5e+04) "None" true))

(fn CalculateForceVector
  (params (Owner :type Wheeled%20Vehicle%20Pawn%20Object%20Reference) (Target :type Wheeled%20Vehicle%20Pawn%20Object%20Reference))
  (Utilities|FlowControl|Sequence
    (:then_0
      (LocalVariables|Set_Owner Owner)
      (LocalVariables|Set_Target Target))
    (:then_1
      (Physics|AddForce (Variables|/Script/ChaosVehicles.WheeledVehiclePawn|GetMesh (LocalVariables|Get_Owner)) (Math|Vector|NegateVector (* (- (Transformation|GetActorLocation (LocalVariables|Get_Owner)) (Transformation|GetActorLocation (LocalVariables|Get_Target))) 2.5)) "None" true)
      (Physics|AddForce (Variables|/Script/ChaosVehicles.WheeledVehiclePawn|GetMesh (LocalVariables|Get_Target)) (* (- (Transformation|GetActorLocation (LocalVariables|Get_Owner)) (Transformation|GetActorLocation (LocalVariables|Get_Target))) 2.5) "None" true)
      (Development|PrintString (Utilities|String|ToString(Vector) (* (- (Transformation|GetActorLocation (LocalVariables|Get_Owner)) (Transformation|GetActorLocation (LocalVariables|Get_Target))) 2.5)) true true "(R=0.000000,G=0.660000,B=1.000000,A=1.000000)" 0.15))))