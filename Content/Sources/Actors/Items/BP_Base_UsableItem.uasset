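; Base usable item actor that other items can derive from, tracking a limited number of uses.
; The OnUse event checks CanUse, which passes while UsesCount is above zero, then calls Use.
; Use decrements UsesCount and briefly prints the item name with the remaining count as a debug log.
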(event Custom|OnUse
  (bind _canuse (CallFunction|CanUse))
  (if _canuse
    (CallFunction|Use)))

(event EventBeginPlay)

(event Collision|EventActorBeginOverlap
  (params (OtherActor :type Actor%20Object%20Reference)))

(event EventTick
  (params (DeltaSeconds :type Float%20%28single-precision%29)))

(fn ConstructionScript)

(fn CanUse
  (return (> (Variables|Default|GetUsesCount) 0)))

(fn Use
  (bind _usescount (Variables|Default|GetUsesCount))
  (Math|Integer|DecrementInt _usescount
    (:%20%20
      ;[1 1 1] Log
      (Development|PrintString (Utilities|String|Append (Utilities|GetDisplayName self) " : " (Utilities|String|ToString(Integer) _usescount)) true true "(R=0.000000,G=0.660000,B=1.000000,A=1.000000)" 0.5))))