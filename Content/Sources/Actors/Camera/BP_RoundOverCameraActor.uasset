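; BP_RoundOverCameraActor is a camera actor for the end of a round that orbits a surviving player.
; SetupCamera takes player controllers, picks the first living BaseController with a valid pawn and attaches itself to that pawn, snapping location but keeping world rotation.
; Tick steadily adds yaw to the root component in world space, so the rig spins around the followed pawn.
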(event EventBeginPlay)

(event Collision|EventActorBeginOverlap
  (params (OtherActor :type Actor%20Object%20Reference)))

(event EventTick
  (params (DeltaSeconds :type Float%20%28single-precision%29))
  (bind _defaultsceneroot (Variables|Default|GetDefaultSceneRoot))
  (bind _returnvalue (Transformation|GetWorldRotation _defaultsceneroot))
  (Transformation|SetWorldRotation (Variables|Default|GetDefaultSceneRoot) (Math|Rotator|MakeRotator (.roll _returnvalue) (.pitch _returnvalue) (+ (.yaw _returnvalue) (* DeltaSeconds 45.0))) false false))

(fn ConstructionScript)

(fn SetupCamera
  (params (PlayerControllers :type Array%20of%20Player%20Controller%20Object%20References))
  (for _array_element PlayerControllers
    (bind _asbase_controller (Utilities|Casting|CastToBaseController _array_element))
    (if (not (Variables|/Game/Sources/Controllers/BaseController.BaseController_C|GetIsDead _asbase_controller))
      (if (Utilities|IsValid (Pawn|GetControlledPawn _asbase_controller))
        (bind _output_get (Variables|Default|SetFollowingActor (Pawn|GetControlledPawn _asbase_controller)))
        (Transformation|AttachActorToActor _output_get "None" "SnapToTarget" "KeepWorld" "KeepRelative" true)
        (return)))))