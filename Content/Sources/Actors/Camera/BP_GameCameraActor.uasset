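; Shared multiplayer camera actor that frames all alive pawns reported by MashedGameMode and eliminates vehicles that leave the screen.
; Each tick it refreshes targets, eases spring arm length toward the clamped largest pairwise player distance, and interpolates toward their average location, adjusting only yaw.
; After a grace period from creation, targets projecting outside the first player's viewport are killed through the game mode.
; SetupCamera seeds the starting position and framing.
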(event EventTick
  (params (DeltaSeconds :type Float%20%28single-precision%29))
  (CallFunction|UpdateTargets)
  (CallFunction|SetArmLength (Variables|Default|GetSpringArmLength_InterpSpeed))
  (CallFunction|SetCameraPosition (Variables|Default|GetCameraLoc_InterpSpeed))
  (CallFunction|KillInvisiblePlayers 1e+01))

(fn ConstructionScript)

(fn CalculateMaxDistance
  (bind _targets (Variables|Default|GetTargets))
  (for (_array_element _array_index) _targets
    (LocalVariables|SetPlayerA _array_element)
    ;[1 1 1] Get all distances between players
    (for _index (range (+ _array_index 1) (- (Utilities|Array|Length _targets) 1))
      (LocalVariables|SetPlayerB (Utilities|Array|Get(acopy) _targets _index))
      (Utilities|Array|Add (LocalVariables|GetDistances) (Transformation|GetDistanceTo (LocalVariables|GetPlayerA) (LocalVariables|GetPlayerB)))))
  (return (.MaxValue (Math|Float|MaxOfFloatArray (LocalVariables|GetDistances)))))

(fn SetArmLength
  (params (SpringArmSpeed :type Float%20%28single-precision%29))
  (bind _springarm (Variables|Default|GetSpringArm))
  (bind _maxvalue (CallFunction|CalculateMaxDistance))
  (Variables|/Script/Engine.SpringArmComponent|SetTargetArmLength _springarm (Math|Interpolation|FInterpTo (Variables|/Script/Engine.SpringArmComponent|GetTargetArmLength _springarm) (Math|Float|Clamp(Float) _maxvalue (Variables|Default|GetMinArmLength) (Variables|Default|GetMaxArmLength)) (Utilities|Time|GetWorldDeltaSeconds) SpringArmSpeed)))

(fn SetCameraPosition
  (params (CameraSpeed :type Float%20%28single-precision%29))
  (bind _returnvalue (Transformation|GetActorRotation))
  (bind _targets (Variables|Default|GetTargets))
  (if (!= 0 (Utilities|Array|Length _targets))
    (for _array_element _targets
      (Utilities|Array|Add (LocalVariables|GetPlayerLocations) (Transformation|GetActorLocation _array_element)))
    (Transformation|SetActorLocation (Math|Interpolation|VInterpTo (Variables|Default|GetPrevCamPos) (Math|Vector|GetVectorArrayAverage (LocalVariables|GetPlayerLocations)) (Utilities|Time|GetWorldDeltaSeconds) CameraSpeed) false false)
    (Variables|Default|SetPrevCamPos (Math|Interpolation|VInterpTo (Variables|Default|GetPrevCamPos) (Math|Vector|GetVectorArrayAverage (LocalVariables|GetPlayerLocations)) (Utilities|Time|GetWorldDeltaSeconds) CameraSpeed))
    (Transformation|SetActorRotation (Math|Rotator|MakeRotator (.roll _returnvalue) (.pitch _returnvalue) (.yaw (Math|Rotator|FindLookatRotation (Transformation|GetWorldLocation (Variables|Default|GetCamera)) (Math|Interpolation|VInterpTo (Variables|Default|GetPrevCamPos) (Math|Vector|GetVectorArrayAverage (LocalVariables|GetPlayerLocations)) (Utilities|Time|GetWorldDeltaSeconds) CameraSpeed)))))
    (Utilities|Array|Clear (LocalVariables|GetPlayerLocations))))

(fn CheckActorVisibility
  (params (Actor :type Actor%20Object%20Reference))
  (bind _returnvalue (Game|GetPlayerController 0))
  (bind _returnvalue_2 (Transformation|GetActorLocation Actor))
  (bind _screenlocation (Class|PlayerController|ProjectWorldLocationtoScreen _returnvalue _returnvalue_2 false))
  (bind (_sizex _sizey) (HUD|GetViewportSize _returnvalue))
  (bind (_x _y) (Math|Vector2D|BreakVector2D _screenlocation))
  (return (Math|Boolean|ANDBoolean (> _x -5.0) (> _y -5.0) (< _x _sizex) (< _y _sizey))))

(fn UpdateTargets
  (bind _asmashed_game_mode (Utilities|Casting|CastToMashedGameMode (Game|GetGameMode)))
  (bind _pawns (Default|GetAlivePawns _asmashed_game_mode))
  (Variables|Default|SetTargets _pawns))

(fn SetupCamera
  (params (PlayerControllers :type Array%20of%20Player%20Controller%20Object%20References))
  (Variables|Default|SetPrevCamPos (Transformation|GetActorLocation))
  (CallFunction|UpdateTargets)
  (CallFunction|SetCameraPosition 1.0)
  (CallFunction|SetArmLength 1.0)
  (Utilities|Casting|CastToMashedGameMode (Game|GetGameMode)))

(fn KillInvisiblePlayers
  (params (SafeTime :type Float%20%28single-precision%29))
  (if (not (< (Actor|GetGameTimeSinceCreation) SafeTime))
    (for _array_element (Variables|Default|GetTargets)
      (bind _isvisible (CallFunction|CheckActorVisibility _array_element))
      (if (not _isvisible)
        (bind _aswheeled_vehicle_pawn (Utilities|Casting|CastToWheeledVehiclePawn _array_element))
        (bind _asmashed_game_mode (Utilities|Casting|CastToMashedGameMode (Game|GetGameMode)))
        (Default|KillPlayer _asmashed_game_mode _aswheeled_vehicle_pawn)))))