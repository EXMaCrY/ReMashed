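; Shared camera actor that frames all players from the game mode's Players list, blending every PlayerController's view to itself shortly after BeginPlay.
; Each tick sets spring arm length from the largest distance between any player pair, clamped to min and max limits.
; It also interpolates its location toward the players' average position and adjusts only yaw to look toward that smoothed point.
; SetCameraRotation is an empty stub.
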(event EventBeginPlay
  (Utilities|FlowControl|Delay 0.2)
  (CallFunction|SetupCamera))

(event EventTick
  (params (DeltaSeconds :type Float%20%28single-precision%29))
  (CallFunction|SetArmLength)
  (CallFunction|SetCameraPosition))

(fn ConstructionScript)

(fn SetupCamera
  (Variables|Default|SetPlayers (Variables|/Game/Sources/GameMode/MashedGameMode.MashedGameMode_C|GetPlayers (.AsMashed%20Game%20Mode (Utilities|Casting|CastToMashedGameMode (Game|GetGameMode)))))
  (bind _outactors (Actor|GetAllActorsOfClass "/Script/Engine.PlayerController"))
  (Game|Player|SetViewTargetwithBlend _outactors self 3.0 "VTBlend_Linear" 0.0 false)
  (Variables|Default|SetPrevCamPos (Transformation|GetActorLocation)))

(fn CalculateMaxDistance
  (bind _players (Variables|Default|GetPlayers))
  (for (_array_element _array_index) _players
    (LocalVariables|SetPlayerA _array_element)
    ;[1 1 1] Get all distances between players
    (for _index (range (+ _array_index 1) (- (Utilities|Array|Length _players) 1))
      (LocalVariables|SetPlayerB (Utilities|Array|Get(acopy) _players _index))
      (Utilities|Array|Add (LocalVariables|GetDistances) (Transformation|GetDistanceTo (LocalVariables|GetPlayerA) (LocalVariables|GetPlayerB)))))
  (return (.MaxValue (Math|Float|MaxOfFloatArray (LocalVariables|GetDistances)))))

(fn SetArmLength
  (bind _maxvalue (CallFunction|CalculateMaxDistance))
  (Variables|/Script/Engine.SpringArmComponent|SetTargetArmLength (Variables|Default|GetSpringArm) (Math|Float|Clamp(Float) _maxvalue (Variables|Default|GetMinArmLength) (Variables|Default|GetMaxArmLength))))

(fn SetCameraPosition
  (bind _returnvalue (Transformation|GetActorRotation))
  (bind _players (Variables|Default|GetPlayers))
  (if (!= 0 (Utilities|Array|Length _players))
    (for _array_element _players
      (Utilities|Array|Add (LocalVariables|GetPlayerLocations) (Transformation|GetActorLocation _array_element)))
    (Transformation|SetActorLocation (Math|Interpolation|VInterpTo (Variables|Default|GetPrevCamPos) (Math|Vector|GetVectorArrayAverage (LocalVariables|GetPlayerLocations)) (Utilities|Time|GetWorldDeltaSeconds) (Variables|Default|GetCameraLoc_InterpSpeed)) true true)
    (Variables|Default|SetPrevCamPos (Math|Interpolation|VInterpTo (Variables|Default|GetPrevCamPos) (Math|Vector|GetVectorArrayAverage (LocalVariables|GetPlayerLocations)) (Utilities|Time|GetWorldDeltaSeconds) (Variables|Default|GetCameraLoc_InterpSpeed)))
    (Transformation|SetActorRotation (Math|Rotator|MakeRotator (.roll _returnvalue) (.pitch _returnvalue) (.yaw (Math|Rotator|FindLookatRotation (Transformation|GetWorldLocation (Variables|Default|GetCamera)) (Math|Interpolation|VInterpTo (Variables|Default|GetPrevCamPos) (Math|Vector|GetVectorArrayAverage (LocalVariables|GetPlayerLocations)) (Utilities|Time|GetWorldDeltaSeconds) (Variables|Default|GetCameraLoc_InterpSpeed))))))
    (Utilities|Array|Clear (LocalVariables|GetPlayerLocations))))

(fn SetCameraRotation)