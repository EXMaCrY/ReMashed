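; Laser sight actor that shows a beam and optionally auto-aims it at pawns.
; Each tick, a visibility trace along the beam's up vector stretches the mesh to the hit or maximum range and stores the point for GetTargetPoint.
; With auto-aim enabled, pawns entering AutoAimMesh become the target, swapping the material and rotating the beam toward their bounds center.
; Any pawn leaving clears the target and restores rotation and material.
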(event OnComponentBeginOverlap(AutoAimMesh)
  (params (OverlappedComponent :type Primitive%20Component%20Object%20Reference) (OtherActor :type Actor%20Object%20Reference) (OtherComp :type Primitive%20Component%20Object%20Reference) (OtherBodyIndex :type Integer) (bFromSweep :type Boolean) (SweepResult :type Hit%20Result%20Structure%20%28by%20ref%29))
  (if (Variables|Default|GetIsAutoAimEnabled)
    (bind _aspawn (Utilities|Casting|CastToPawn OtherActor))
    (Variables|Default|SetTarget _aspawn)
    (Rendering|Material|SetMaterial (Variables|Default|GetLaserSight) 0 "/Game/Resources/Materials/Laser/LaserPointerMaterialInst.LaserPointerMaterialInst")))

(event OnComponentEndOverlap(AutoAimMesh)
  (params (OverlappedComponent :type Primitive%20Component%20Object%20Reference) (OtherActor :type Actor%20Object%20Reference) (OtherComp :type Primitive%20Component%20Object%20Reference) (OtherBodyIndex :type Integer))
  (Utilities|Casting|CastToPawn OtherActor)
  (Variables|Default|SetTarget 0)
  (Transformation|SetRelativeRotation (Variables|Default|GetLaserSight) (Variables|Default|GetBaseLaserRotation) false false)
  (Rendering|Material|SetMaterial (Variables|Default|GetLaserSight) 0 "/Game/Resources/Materials/Laser/LaserPointerMaterial_Inst.LaserPointerMaterial_Inst"))

(event EventBeginPlay
  (Variables|Default|SetBaseLaserRotation (Variables|/Script/Engine.SceneComponent|GetRelativeRotation (Variables|Default|GetLaserSight))))

(event Collision|EventActorBeginOverlap
  (params (OtherActor :type Actor%20Object%20Reference)))

(event EventTick
  (params (DeltaSeconds :type Float%20%28single-precision%29))
  (CallFunction|LineTraceforLaserSight)
  (if (Variables|Default|GetIsAutoAimEnabled)
    (if (Utilities|IsValid (Variables|Default|GetTarget))
      (Transformation|SetWorldRotation (Variables|Default|GetLaserSight) (Math|Rotator|CombineRotators (Variables|Default|GetBaseLaserRotation) (Math|Rotator|FindLookatRotation (Transformation|GetWorldLocation (Variables|Default|GetLaserSight)) (.Origin (Collision|GetActorBounds (Variables|Default|GetTarget) true false)))) false false))))

(fn ConstructionScript)

(fn LineTraceforLaserSight
  (bind _lasersight (Variables|Default|GetLaserSight))
  (bind _returnvalue (Transformation|GetWorldLocation _lasersight))
  (bind _returnvalue_2 (Math|Vector|GetUpVector _lasersight))
  (bind _returnvalue_3 (* _returnvalue_2 1e+04))
  (bind _returnvalue_4 (+ _returnvalue _returnvalue_3))
  (bind (_outhit _returnvalue_5) (Collision|LineTraceByChannel _returnvalue _returnvalue_4 "TraceTypeQuery1" false 0 "None"))
  (if _returnvalue_5
    (Variables|Default|SetTargetPoint (.Location (Collision|BreakHitResult _outhit)))
    (Transformation|SetWorldScale3D (Variables|Default|GetLaserSight) (Math|Vector|MakeVector 0.03 0.03 (/ (Math|Vector|VectorLength (- (.Location (Collision|BreakHitResult _outhit)) (.TraceStart (Collision|BreakHitResult _outhit)))) 1e+02)))
    (else
      (Variables|Default|SetTargetPoint _returnvalue_4)
      (Transformation|SetWorldScale3D (Variables|Default|GetLaserSight) "0.030000,0.030000,100.000000"))))

(fn GetTargetPoint
  (return (Variables|Default|GetTargetPoint)))