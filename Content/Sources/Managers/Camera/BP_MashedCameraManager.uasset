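; BP_MashedCameraManager is a manager Blueprint that owns the active gameplay camera and handles switching between camera classes.
; SetupCameraManager stores the PlayerControllers that the cameras serve.
; SwitchCamera destroys the current camera, spawns the requested class at a given transform, sets it as their view target, and passes them to BP_BaseCameraActor's SetupCamera.
; DestroyCamera removes the current camera.
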(event EventBeginPlay)

(event Collision|EventActorBeginOverlap
  (params (OtherActor :type Actor%20Object%20Reference)))

(event EventTick
  (params (DeltaSeconds :type Float%20%28single-precision%29)))

(fn ConstructionScript)

(fn SetupCameraManager
  (params (PlayerControllers :type Array%20of%20Player%20Controller%20Object%20References))
  (Variables|Default|SetPlayerControllers PlayerControllers))

(fn SwitchCamera
  (params (CameraClass :type Actor%20Class%20Reference) (SpawnTransform :type Transform))
  (if (Utilities|IsValid (Variables|Default|GetCurrentCamera))
    (Actor|DestroyActor (Variables|Default|GetCurrentCamera)))
  (bind _returnvalue (Game|SpawnActorfromClass CameraClass SpawnTransform "AlwaysSpawn" 0 0))
  (bind _output_get (Variables|Default|SetCurrentCamera _returnvalue))
  (Game|Player|SetViewTargetwithBlend (Variables|Default|GetPlayerControllers) _output_get 0.0 "VTBlend_Linear" 0.0 false)
  (bind _asbp_base_camera_actor (Utilities|Casting|CastToBP_BaseCameraActor _returnvalue))
  (Default|SetupCamera _asbp_base_camera_actor (Variables|Default|GetPlayerControllers)))

(fn DestroyCamera
  (Actor|DestroyActor (Variables|Default|GetCurrentCamera)))